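; Game state for a soccer match that tracks both teams' scores and triggers the game-over UI.
; BeginPlay adds the player HUD widget to the viewport.
; AddScoreToTeam increments Team A or Team B's score unless the match has ended.
; Once the match has ended, HandleGameOverUI passes that state to player 0's third-person character through MulticastHandleGameOver.
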(event `self.ReceiveBeginPlay`
  ; Adding Crossair to Viewport
  (bind _returnvalue (`|CreateWidget` "/Game/Assets/Blueprints/UI/WP_PlayerHUD.WP_PlayerHUD_C"))
  (`UserWidget.AddToViewport` _returnvalue 0))

(event `AddScoreToTeam`
  (params (isTeamA :type Boolean))
  ; Handle Score Increment to UI
  (if (`self.isMatchEnded`)
    (`KismetSystemLibrary.PrintString` "NoScoreIncrement")
    (elif isTeamA
      (`/Engine/EditorBlueprintResources/StandardMacros.IncrementInt` (`self.teamAScore`))
      (else
        (`/Engine/EditorBlueprintResources/StandardMacros.IncrementInt` (`self.teamBScore`))))))

(event `HandleGameOverUI`
  (bind _ismatchended (`self.isMatchEnded`))
  ; Handle Game Over
  (if _ismatchended
    (bind _asbp_third_person_character (cast `/Game/ThirdPerson/Blueprints/BP_ThirdPersonCharacter` (`GameplayStatics.GetPlayerCharacter` 0)))
    (`/Game/ThirdPerson/Blueprints/BP_ThirdPersonCharacter.Multicast_HandleGameOver` _asbp_third_person_character _ismatchended)))

(fn `UserConstructionScript`)