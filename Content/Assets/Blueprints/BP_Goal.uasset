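; Goal trigger Blueprint that detects a football entering its box and registers the score.
; On authority, overlaps with BPI_Football actors pass the scoring side to the game mode, which handles scoring and ball respawn.
; Multicasts notify the ball, randomize the goal's dynamic material color and fire a delayed Niagara celebration.
; A timeline bounces the goal mesh up and back, multicasting its height on each update.
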(event `self.ReceiveBeginPlay`
  ; Creating Dynamic Material Instance
  (`self.CreateDynamicMaterialInst`))

(event `self.Box.OnComponentBeginOverlap`
  (params (OverlappedComponent :type "PrimitiveComponent Object Reference") (OtherActor :type "Actor Object Reference") (OtherComp :type "PrimitiveComponent Object Reference") (OtherBodyIndex :type Integer) (bFromSweep :type Boolean) (SweepResult :type "HitResult Structure (by ref)"))
  (bind _isscoringteamside (`self.isScoringTeamSide`))
  ; Goal Overlap Functionality
  (`/Engine/EditorBlueprintResources/ActorMacros.Switch Has Authority`
    (:`Authority`
      (if (`KismetSystemLibrary.DoesImplementInterface` OtherActor "/Game/Assets/Blueprints/Interfaces/BPI_Football.BPI_Football_C")
        (`self.Multicast_HandleOnScore` OtherActor)
        (bind _asbp_third_person_game_mode (cast `/Game/ThirdPerson/Blueprints/BP_ThirdPersonGameMode` (`GameplayStatics.GetGameMode`)))
        (set `/Game/ThirdPerson/Blueprints/BP_ThirdPersonGameMode.isScoringTeam` _isscoringteamside _asbp_third_person_game_mode)
        (`/Game/ThirdPerson/Blueprints/BP_ThirdPersonGameMode.HandleGoalScored` _asbp_third_person_game_mode)
        (`self.Multicast_GoalCelebration`)
        (`self.Multicast_HandleGoalColorChange` _isscoringteamside (`KismetMathLibrary.RandomFloat`) (`KismetMathLibrary.RandomFloat`) (`KismetMathLibrary.RandomFloat`))
        (`self.Multicast_MoveGoalUp`)
        (`/Game/ThirdPerson/Blueprints/BP_ThirdPersonGameMode.Server_HandleBallRespawn` _asbp_third_person_game_mode)))))

(event `Multicast_HandleOnScore`
  (params (actorTarget :type "Actor Object Reference"))
  ; Remote Procedure Calls
  (message `/Game/Assets/Blueprints/Interfaces/BPI_Football.OnScored` actorTarget))

(event `Multicast_HandleGoalColorChange`
  (params (teamSide :type Boolean) (r :type "Float (double-precision)") (g :type "Float (double-precision)") (b :type "Float (double-precision)"))
  ; Remote Procedure Calls
  (`self.HandleGoalColorChange` teamSide r g b))

(event `Multicast_TriggerAnimation`
  (params (zAxis :type "Float (double-precision)") (goalMeshSceneComponent :type "SceneComponent Object Reference"))
  ; Remote Procedure Calls
  (`SceneComponent.K2_SetRelativeLocation` goalMeshSceneComponent (`KismetMathLibrary.MakeVector` 0.0 0.0 zAxis) false false))

(event `Multicast_GoalCelebration`
  ; Remote Procedure Calls
  (`KismetSystemLibrary.Delay` 1.0)
  (`self.PlayGoalCelebration`))

(event `Multicast_MoveGoalUp`
  ; Goal Jump Animation Timeline
  (bind (_direction _movegoalposition) (`Timeline|Goal Animation` :!label _label)
    (:`Update`
      (`self.Multicast_TriggerAnimation` (* _movegoalposition (`self.maxJumpHeight`)) (`StaticMeshActor.StaticMeshComponent` (`self.goalMesh`))))
    (:`Finished`
      (`self.Multicast_MoveGoalDown`))))

(event `Multicast_MoveGoalDown`
  ; Goal Jump Animation Timeline
  (goto _label :!via `Reverse`))

(fn `CreateDynamicMaterialInst`
  (bind _returnvalue (`PrimitiveComponent.CreateDynamicMaterialInstance` (`StaticMeshActor.StaticMeshComponent` (`self.goalMesh`)) 0 null "None"))
  (set `self.goalMID` _returnvalue))

(fn `HandleGoalColorChange`
  (params (isTeamA :type Boolean) (r :type "Float (double-precision)") (g :type "Float (double-precision)") (b :type "Float (double-precision)"))
  (if isTeamA
    _
    (else
      _))
  (`MaterialInstanceDynamic.SetVectorParameterValue` (`self.goalMID`) "Color" (make `LinearColor` r g b)))

(fn `PlayGoalCelebration`
  (bind _niagara (`self.Niagara`))
  (`/Engine/EditorBlueprintResources/StandardMacros.IsValid` _niagara
    (:`Is Valid`
      (`ActorComponent.Activate` _niagara true))
    (:`Is Not Valid`
      (`KismetSystemLibrary.PrintString` "No Celebration added"))))

(fn `UserConstructionScript`)